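; BPA_CityBuilding1 is a city building actor with a randomised colour and switchable lighting.
; The construction script picks a colour from BuildingColours for a dynamic M_Basic material on slot 1, then calls SetLighting.
; SetLighting stores LightsOn, then either applies a light material to slot 2 and powers two rect lights, or matches that slot to the building colour and zeroes their intensity.
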(event EventBeginPlay)

(event Collision|EventActorBeginOverlap
  (params (OtherActor :type Actor%20Object%20Reference)))

(event EventTick
  (params (DeltaSeconds :type Float%20%28single-precision%29)))

(fn ConstructionScript
  (bind _buildingcolours (Variables|Default|GetBuildingColours))
  (bind _returnvalue (Rendering|Material|CreateDynamicMaterialInstance (Variables|Default|GetStaticMesh) 1 "/Game/Environment/Materials/M_Basic.M_Basic" "None" :!class /Script/Engine.PrimitiveComponent))
  (bind _output_get (Variables|Default|SetBuildingColour (Utilities|Array|Get(acopy) _buildingcolours (Math|Random|RandomInteger (Utilities|Array|Length _buildingcolours)))))
  (Rendering|Material|SetVectorParameterValue _returnvalue "BaseColor" (Math|Conversions|ToLinearColor(Color) _output_get) :!class /Script/Engine.MaterialInstanceDynamic)
  (CallFunction|SetLighting (Variables|Default|GetLightsOn)))

(fn SetLighting
  (params (LightsOn :type Boolean))
  (bind _output_get (Variables|Default|SetLightsOn LightsOn))
  (if _output_get
    (Rendering|Material|SetMaterial (Variables|Default|GetStaticMesh) 2 "/Game/Environment/Materials/MI_Light_Dimmer.MI_Light_Dimmer")
    (Rendering|Components|Light|SetIntensity (Variables|Default|GetRectLight1) 7e+03)
    (else
      (bind _returnvalue (Rendering|Material|CreateDynamicMaterialInstance (Variables|Default|GetStaticMesh) 2 "/Game/Environment/Materials/M_Basic.M_Basic" "None" :!class /Script/Engine.PrimitiveComponent))
      (Rendering|Material|SetVectorParameterValue _returnvalue "BaseColor" (Math|Conversions|ToLinearColor(Color) (Variables|Default|GetBuildingColour)) :!class /Script/Engine.MaterialInstanceDynamic)
      (Rendering|Components|Light|SetIntensity (Variables|Default|GetRectLight1) 0.0))))