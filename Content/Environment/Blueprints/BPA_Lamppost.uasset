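; BPA_Lamppost is a lamppost actor whose light can be switched on or off through a LightsOn flag.
; The construction script passes that flag to SetLighting, which stores it and updates the mesh and point light together.
; When on, the second material slot uses a light material and the point light is bright; when off, it uses basic metal and zero intensity.
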(event EventBeginPlay)

(event Collision|EventActorBeginOverlap
  (params (OtherActor :type Actor%20Object%20Reference)))

(event EventTick
  (params (DeltaSeconds :type Float%20%28single-precision%29)))

(fn ConstructionScript
  (CallFunction|SetLighting (Variables|Default|GetLightsOn)))

(fn SetLighting
  (params (LightsOn :type Boolean))
  (bind _output_get (Variables|Default|SetLightsOn LightsOn))
  (if _output_get
    (Rendering|Material|SetMaterial (Variables|Default|GetStaticMesh) 1 "/Game/Environment/Materials/MI_Light_Dimmer.MI_Light_Dimmer")
    (Rendering|Components|Light|SetIntensity (Variables|Default|GetPointLight) 5e+03)
    (else
      (Rendering|Material|SetMaterial (Variables|Default|GetStaticMesh) 1 "/Game/Environment/Materials/MI_Basic_Metal.MI_Basic_Metal")
      (Rendering|Components|Light|SetIntensity (Variables|Default|GetPointLight) 0.0))))