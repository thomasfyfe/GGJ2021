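; BP_PottedTarget is a pot target that reacts to rain and changes the game's happiness score.
; Its RainDetector overlap accepts only actors of class BP_Rain, and a DoOnce lets the reaction run a single time.
; That reaction calls UpdateMood, swaps the Pot mesh to SM_ParkBench, then adds PointsAffect to Happiness on BP_Gamemode.
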(event OnComponentBeginOverlap(RainDetector)
  (params (OverlappedComponent :type Primitive%20Component%20Object%20Reference) (OtherActor :type Actor%20Object%20Reference) (OtherComp :type Primitive%20Component%20Object%20Reference) (OtherBodyIndex :type Integer) (bFromSweep :type Boolean) (SweepResult :type Hit%20Result%20Structure%20%28by%20ref%29))
  (if (== (Utilities|GetClass OtherActor) "/Game/TopDownBP/Blueprints/BP_Rain.BP_Rain_C")
    (Utilities|FlowControl|DoOnce false
      (:Completed
        (CallFunction|UpdateMood)
        (Components|StaticMesh|SetStaticMesh (Variables|Default|GetPot) "/Game/Environment/Meshes/SM_ParkBench.SM_ParkBench")
        (bind _asbp_gamemode (Utilities|Casting|CastToBP_Gamemode (Game|GetGameMode)))
        (Variables|/Game/TopDownBP/Blueprints/BP_Gamemode.BP_Gamemode_C|SetHappiness _asbp_gamemode (+ (Variables|/Game/TopDownBP/Blueprints/BP_Gamemode.BP_Gamemode_C|GetHappiness _asbp_gamemode) (Variables|Default|GetPointsAffect)))))))

(fn ConstructionScript)